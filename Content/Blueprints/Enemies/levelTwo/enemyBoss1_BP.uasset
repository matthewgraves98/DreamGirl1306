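; Level-two 2D boss enemy that fires projectiles and damages zeke_BP on contact, and dies when its health runs out.
; While Zeke is inside Sphere1, Tick spawns a projectile at a fixed offset, using a Delay both as cooldown and projectile lifetime.
; Hits apply time-gated damage and launch Zeke by the IsFacingRight flag.
; The outer Sphere's chase logic is disconnected, and animation always uses the idle flipbook.
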(event `self.ReceiveTick`
  (params (DeltaSeconds :type "Float (single-precision)"))
  ;[1 1 1] Tick
  (`self.UpdateAnimation`)
  (if (`self.isOverlappingForCombat`)
    (if (not (`self.cooldownActive`))
      (set `self.cooldownActive` true)
      (bind _returnvalue (`|SpawnActorFromClass` "/Game/Blueprints/Enemies/levelTwo/enemyProjectile_Bp.enemyProjectile_BP_C" (`KismetMathLibrary.MakeTransform` (+ (`self.K2_GetActorLocation`) (25.0 0.0 -180.0) (0.0 0.0 0.0)) (struct :`Yaw` 180.0) (0.7 0.7 0.7)) "Undefined" "OverrideRootScale" null null))
      (`KismetSystemLibrary.Delay` 2.0)
      (set `self.cooldownActive` false)
      (`self.K2_DestroyActor` _returnvalue))))

(event `self.ReceiveBeginPlay`
  ;[1 1 1] Begin Play
  (set `self.CurrentHealth` (`self.MaxHealth`)))

(event `self.ReceiveHit`
  (params (MyComp :type "PrimitiveComponent Object Reference") (Other :type "Actor Object Reference") (OtherComp :type "PrimitiveComponent Object Reference") (bSelfMoved :type Boolean) (HitLocation :type "Vector Structure") (HitNormal :type "Vector Structure") (NormalImpulse :type "Vector Structure") (Hit :type "HitResult Structure (by ref)"))
  ;[1 1 1] Apply Damage
  (`/Engine/EditorBlueprintResources/StandardMacros.CompareFloat` (`self.AttackCooldown`) (`KismetSystemLibrary.GetGameTimeInSeconds`)
    (:`<`
      (bind _aszeke_bp (cast `/Game/Blueprints/Zeke/zeke_BP` Other))
      (`GameplayStatics.ApplyDamage` _aszeke_bp (`self.Damage`))
      (set `self.AttackCooldown` (+ (`KismetSystemLibrary.GetGameTimeInSeconds`) 1.0))
      (if (`self.isFacingRight`)
        (`self.LaunchCharacter` _aszeke_bp (+ (* (`self.GetActorForwardVector`) 500.0) (* (`self.GetActorUpVector`) 250.0)) false false)
        (else
          (`self.LaunchCharacter` _aszeke_bp (+ (* (`self.GetActorForwardVector`) -500.0) (* (`self.GetActorUpVector`) 250.0)) false false))))))

(event `self.Sphere.OnComponentBeginOverlap`
  (params (OverlappedComponent :type "PrimitiveComponent Object Reference") (OtherActor :type "Actor Object Reference") (OtherComp :type "PrimitiveComponent Object Reference") (OtherBodyIndex :type Integer) (bFromSweep :type Boolean) (SweepResult :type "HitResult Structure (by ref)"))
  ;[1 1 1] Character in Range
  (cast `/Game/Blueprints/Zeke/zeke_BP` OtherActor)
  (set `self.isOverlapping` true))

(event `self.Sphere1.OnComponentBeginOverlap`
  (params (OverlappedComponent :type "PrimitiveComponent Object Reference") (OtherActor :type "Actor Object Reference") (OtherComp :type "PrimitiveComponent Object Reference") (OtherBodyIndex :type Integer) (bFromSweep :type Boolean) (SweepResult :type "HitResult Structure (by ref)"))
  ;[1 1 1] overlappingForCombat
  (cast `/Game/Blueprints/Zeke/zeke_BP` OtherActor)
  (set `self.isOverlappingForCombat` true)
  (`KismetSystemLibrary.Delay` 1.0)
  (set `self.isOverlapping` false))

(event `self.Sphere.OnComponentEndOverlap`
  (params (OverlappedComponent :type "PrimitiveComponent Object Reference") (OtherActor :type "Actor Object Reference") (OtherComp :type "PrimitiveComponent Object Reference") (OtherBodyIndex :type Integer))
  ;[1 1 1] Character in Range
  (cast `/Game/Blueprints/Zeke/zeke_BP` OtherActor)
  (set `self.isOverlapping` false))

(event `self.Sphere1.OnComponentEndOverlap`
  (params (OverlappedComponent :type "PrimitiveComponent Object Reference") (OtherActor :type "Actor Object Reference") (OtherComp :type "PrimitiveComponent Object Reference") (OtherBodyIndex :type Integer))
  ;[1 1 1] overlappingForCombat
  (cast `/Game/Blueprints/Zeke/zeke_BP` OtherActor)
  (set `self.isOverlappingForCombat` false))

(event `UpdateAnimation`
  ;[1 1 1] Update Animation
  (`PaperFlipbookComponent.SetFlipbook` (`self.Sprite`) (select `bool` (> (`KismetMathLibrary.VSize` (`self.GetVelocity`)) 0.0) :`false` "/Game/FlipBooks/bossIdleFlip.bossIdleFlip" :`true` "/Game/FlipBooks/bossIdleFlip.bossIdleFlip" :!type "PaperFlipbook Object Reference")))

(event `self.ReceiveAnyDamage`
  (params (Damage :type "Float (single-precision)") (DamageType :type "DamageType Object Reference") (InstigatedBy :type "Controller Object Reference") (DamageCauser :type "Actor Object Reference"))
  ;[1 1 1] Recieve Damage
  (bind _output_get (set `self.CurrentHealth` (- (`self.CurrentHealth`) Damage)))
  (if (<= (`self.CurrentHealth`) 0.0)
    (`self.K2_DestroyActor`)))

(fn `UserConstructionScript`)