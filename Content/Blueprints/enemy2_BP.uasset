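; Paper2D enemy character that chases the player (zeke_BP) along the X axis while the player is inside its detection sphere, showing an angry flipbook.
; On hit, it damages and launches the player, limited by a game-time cooldown.
; Incoming damage lowers health; at zero it spawns a random health or energy pickup or power-down, then destroys itself.
; The combat-range sphere and movement-direction flag are set but not read here.
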(event `self.ReceiveTick`
  (params (DeltaSeconds :type "Float (single-precision)"))
  (bind _returnvalue_x (`KismetMathLibrary.BreakVector` (`SceneComponent.K2_GetComponentLocation` (`self.CapsuleComponent`))))
  ;[1 1 1] Tick
  (`self.UpdateAnimation`)
  (if (`self.isOverlapping`)
    (`PaperFlipbookComponent.SetFlipbook` (`self.Sprite`) "/Game/FlipBooks/enemyAngryFlip.enemyAngryFlip")
    (bind _aszeke_bp (cast `/Game/Blueprints/Zeke/zeke_BP` (`GameplayStatics.GetPlayerCharacter` 0)))
    (bind _returnvalue_x_2 (`KismetMathLibrary.BreakVector` (`SceneComponent.K2_GetComponentLocation` (`Character.CapsuleComponent` _aszeke_bp))))
    (bind _returnvalue (- _returnvalue_x_2 _returnvalue_x))
    (if (>= _returnvalue 0.0)
      (set `self.BisMovingRight` true)
      (else
        (set `self.BisMovingRight` false)))
    (`self.AddMovementInput` (1.0 0.0 0.0) _returnvalue)))

(event `self.ReceiveBeginPlay`
  ;[1 1 1] Begin Play
  (set `self.CurrentHealth` (`self.MaxHealth`)))

(event `self.ReceiveHit`
  (params (MyComp :type "PrimitiveComponent Object Reference") (Other :type "Actor Object Reference") (OtherComp :type "PrimitiveComponent Object Reference") (bSelfMoved :type Boolean) (HitLocation :type "Vector Structure") (HitNormal :type "Vector Structure") (NormalImpulse :type "Vector Structure") (Hit :type "HitResult Structure (by ref)"))
  ;[1 1 1] Apply Damage
  (`/Engine/EditorBlueprintResources/StandardMacros.CompareFloat` (`self.AttackCooldown`) (`KismetSystemLibrary.GetGameTimeInSeconds`)
    (:`<`
      (bind _aszeke_bp (cast `/Game/Blueprints/Zeke/zeke_BP` Other))
      (`GameplayStatics.ApplyDamage` _aszeke_bp (`self.Damage`))
      (set `self.AttackCooldown` (+ (`KismetSystemLibrary.GetGameTimeInSeconds`) 1.0))
      (`self.LaunchCharacter` _aszeke_bp (+ (* (`self.GetActorForwardVector`) -500.0) (* (`self.GetActorUpVector`) 250.0)) false false))))

(event `self.Sphere.OnComponentBeginOverlap`
  (params (OverlappedComponent :type "PrimitiveComponent Object Reference") (OtherActor :type "Actor Object Reference") (OtherComp :type "PrimitiveComponent Object Reference") (OtherBodyIndex :type Integer) (bFromSweep :type Boolean) (SweepResult :type "HitResult Structure (by ref)"))
  ;[1 1 1] Character in Range
  (cast `/Game/Blueprints/Zeke/zeke_BP` OtherActor)
  (set `self.isOverlapping` true))

(event `self.Sphere1.OnComponentBeginOverlap`
  (params (OverlappedComponent :type "PrimitiveComponent Object Reference") (OtherActor :type "Actor Object Reference") (OtherComp :type "PrimitiveComponent Object Reference") (OtherBodyIndex :type Integer) (bFromSweep :type Boolean) (SweepResult :type "HitResult Structure (by ref)"))
  ;[1 1 1] In Combat Range
  (cast `/Game/Blueprints/Zeke/zeke_BP` OtherActor)
  (set `self.overlappingForCombat` true))

(event `self.Sphere.OnComponentEndOverlap`
  (params (OverlappedComponent :type "PrimitiveComponent Object Reference") (OtherActor :type "Actor Object Reference") (OtherComp :type "PrimitiveComponent Object Reference") (OtherBodyIndex :type Integer))
  ;[1 1 1] Character in Range
  (cast `/Game/Blueprints/Zeke/zeke_BP` OtherActor)
  (set `self.isOverlapping` false))

(event `self.Sphere1.OnComponentEndOverlap`
  (params (OverlappedComponent :type "PrimitiveComponent Object Reference") (OtherActor :type "Actor Object Reference") (OtherComp :type "PrimitiveComponent Object Reference") (OtherBodyIndex :type Integer))
  ;[1 1 1] In Combat Range
  (cast `/Game/Blueprints/Zeke/zeke_BP` OtherActor)
  (set `self.overlappingForCombat` false))

(event `UpdateAnimation`
  ;[1 1 1] Update Animation
  (`PaperFlipbookComponent.SetFlipbook` (`self.Sprite`) (select `bool` (> (`KismetMathLibrary.VSize` (`self.GetVelocity`)) 0.0) :`false` "/Game/FlipBooks/EnemyFlip.enemyFlip" :`true` "/Game/FlipBooks/EnemyFlip.enemyFlip" :!type "PaperFlipbook Object Reference")))

(event `self.ReceiveAnyDamage`
  (params (Damage :type "Float (single-precision)") (DamageType :type "DamageType Object Reference") (InstigatedBy :type "Controller Object Reference") (DamageCauser :type "Actor Object Reference"))
  ;[1 1 1] Recieve Damage
  (bind _output_get (set `self.CurrentHealth` (- (`self.CurrentHealth`) Damage)))
  (if (<= (`self.CurrentHealth`) 0.0)
    (switch `int` (`KismetMathLibrary.RandomIntegerInRange` 0 3)
      (:`0`
        (`|SpawnActorFromClass` "/Game/Blueprints/Pickups/healthPickup_BP.healthPickup_BP_C" (`self.GetTransform`) "Undefined" "OverrideRootScale" null null))
      (:`1`
        (`|SpawnActorFromClass` "/Game/Blueprints/Pickups/healthPowerDown_BP.healthPowerDown_BP_C" (`self.GetTransform`) "Undefined" "OverrideRootScale" null null))
      (:`2`
        (`|SpawnActorFromClass` "/Game/Blueprints/Pickups/energyPickup_BP.energyPickup_BP_C" (`self.GetTransform`) "Undefined" "OverrideRootScale" null null))
      (:`3`
        (`|SpawnActorFromClass` "/Game/Blueprints/Pickups/energyPowerDown_BP.energyPowerDown_BP_C" (`self.GetTransform`) "Undefined" "OverrideRootScale" null null)))
    (`self.K2_DestroyActor`)))

(fn `UserConstructionScript`)